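; Black hole actor that pulls physics-simulating components toward itself and destroys those that reach its core.
; Each tick, ApplyFoces pushes components inside GravityInfluence toward the center, with linear distance falloff and stronger vertical pull.
; Killzone overlaps destroy the simulating object's actor and pass its mass to MassGained.
; MassGained computes a new scale, but its timeline sets Sphere scale to zero because the Ease interpolation is unconnected.
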(event `self.ReceiveTick`
  (params (DeltaSeconds :type "Float (single-precision)"))
  (`self.ApplyFoces`))

(event `self.Killzone.OnComponentBeginOverlap`
  (params (OverlappedComponent :type "PrimitiveComponent Object Reference") (OtherActor :type "Actor Object Reference") (OtherComp :type "PrimitiveComponent Object Reference") (OtherBodyIndex :type Integer) (bFromSweep :type Boolean) (SweepResult :type "HitResult Structure (by ref)"))
  (if (`SceneComponent.IsSimulatingPhysics` OtherComp "None")
    (`self.MassGained` (`PrimitiveComponent.GetMass` OtherComp))
    (`self.K2_DestroyActor` OtherActor)))

(event `MassGained`
  (params (Mass :type "Float (double-precision)"))
  (set `self.CurrentScale` (`SceneComponent.K2_GetComponentScale` (`self.Sphere`)))
  (set `self.NewScale` (/ (`self.CurrentScale`) (* Mass (`self.GrowthRate`))))
  (bind (_direction _alpha) (`Timeline|Timeline` :!via `PlayFromStart`)
    (:`Update`
      (`SceneComponent.SetWorldScale3D` (`self.Sphere`) (0.0 0.0 0.0)))))

(fn `ApplyFoces`
  (bind _returnvalue (`self.K2_GetActorLocation`))
  (for _array_element (`PrimitiveComponent.GetOverlappingComponents` (`self.GravityInfluence`))
    (if (`SceneComponent.IsSimulatingPhysics` _array_element "None")
      (bind _returnvalue_2 (`SceneComponent.K2_GetComponentLocation` _array_element))
      (`PrimitiveComponent.AddForce` _array_element (* (`KismetMathLibrary.GetDirectionUnitVector` _returnvalue_2 _returnvalue) (* (- 1.0 (`KismetMathLibrary.FClamp` (/ (`KismetMathLibrary.Vector_Distance` _returnvalue_2 _returnvalue) 5000.0))) 5000.0) (1.0 1.0 5.0) (`self.GravityStrenght`)) "None" false))))

(fn `UserConstructionScript`)