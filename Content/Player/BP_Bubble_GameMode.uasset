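; Game mode for the Bubble game that, on player login, spawns and possesses characters at tagged PlayerStart actors.
; PostLogin creates an additional local player, then switches on that player's controller ID to choose a start tag, with the logging-in controller possessing the spawned pawn.
; Only IDs 0 and 1 reach spawning, and the first has no class set.
; Spawn logic for the third and fourth starts is disconnected.
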(event `self.K2_PostLogin`
  (params (NewPlayer :type "PlayerController Object Reference"))
  (bind _returnvalue (`GameplayStatics.CreatePlayer` -1))
  (switch `int` (`GameplayStatics.GetPlayerControllerID` _returnvalue)
    (:`Default`
      (bind _outactors (`GameplayStatics.GetAllActorsOfClassWithTag` "/Script/Engine.PlayerStart" "PlayerStart4")))
    (:`0`
      (bind _outactors_2 (`GameplayStatics.GetAllActorsOfClassWithTag` "/Script/Engine.PlayerStart" "PlayerStart1"))
      (bind _returnvalue_2 (`|SpawnActorFromClass` "/Game/TopDown/Blueprints/BP_TopDownCharacter.BP_TopDownCharacter_C" (`self.GetTransform` (`|GetArrayItem` _outactors_2)) "Undefined" "MultiplyWithRoot" null null))
      (`Controller.Possess` NewPlayer _returnvalue_2))
    (:`1`
      (bind _outactors_3 (`GameplayStatics.GetAllActorsOfClassWithTag` "/Script/Engine.PlayerStart" "PlayerStart2"))
      (bind _returnvalue_3 (`|SpawnActorFromClass` "/Game/TopDown/Blueprints/BP_TopDownCharacter.BP_TopDownCharacter_C" (`self.GetTransform` (`|GetArrayItem` _outactors_3)) "Undefined" "MultiplyWithRoot" null null))
      (`Controller.Possess` NewPlayer _returnvalue_3))
    (:`2`
      (bind _outactors_4 (`GameplayStatics.GetAllActorsOfClassWithTag` "/Script/Engine.PlayerStart" "PlayerStart3")))))

(fn `UserConstructionScript`)