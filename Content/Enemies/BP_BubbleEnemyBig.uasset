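; BP_BubbleEnemyBig is a large bubble enemy that pulses in size and is meant to split when shot.
; BeginPlay sets a random material, using the random index as the element slot, then starts a self-recalling Pulse timeline that scales the mesh.
; Projectile overlap calls OnHit and Split, but Split's loop body is empty.
; The logic spawning BP_BubbleEnemySmall children and calling OnDeath is disconnected, so hits neither split nor destroy it.
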(event `self.ReceiveBeginPlay`
  (bind (_outitem _outindex) (`KismetArrayLibrary.Array_Random` (`|MakeArray` (`self.Material 1`) (`self.Material 2`) (`self.Material 3`))))
  (`PrimitiveComponent.SetMaterial` (`self.Bubble`) _outindex _outitem)
  (`KismetSystemLibrary.Delay` 0.2)
  (`self.Pulsate`))

(event `Pulsate`
  ; Animation
  (bind (_direction _pulse) (`Timeline|Pulse`)
    (:`Update`
      (`SceneComponent.SetRelativeScale3D` (`self.Bubble`) (`KismetMathLibrary.Conv_DoubleToVector` (`KismetMathLibrary.Lerp` 1.0 2.0 _pulse)))
      (`self.Pulsate`))))

(event `self.Sphere.OnComponentBeginOverlap`
  (params (OverlappedComponent :type "PrimitiveComponent Object Reference") (OtherActor :type "Actor Object Reference") (OtherComp :type "PrimitiveComponent Object Reference") (OtherBodyIndex :type Integer) (bFromSweep :type Boolean) (SweepResult :type "HitResult Structure (by ref)"))
  ; Hit
  (cast `/Game/Player/BP_Projectile` OtherActor)
  (`self.OnHit`))

(event `OnHit`
  ; On Death
  (`self.Split`))

(event `OnDeath`
  ; On Death
  (`self.K2_DestroyActor`))

(event `Split`
  ; On Death
  (for _ (`|MakeArray` (`self.ChildCount`))
    _))

(fn `UserConstructionScript`)