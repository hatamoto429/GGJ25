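; BP_BubbleEnemy is an enemy Blueprint that appears intended to split into copies of itself on death.
; The IA_Shoot input event deducts Damage through ACHealthComponent, then calls OnDeath without checking remaining health.
; OnDeath spawns BP_BubbleEnemy at its own location while Successors is zero or less, decrementing it each pass, so that loop has no exit once entered.
; BeginPlay and the construction script are empty.
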(event `EnhancedInput|/Game/Player/Controls/IA_Shoot`
  (params (ActionValue :type Boolean) (ElapsedSeconds :type "Float (double-precision)") (TriggeredSeconds :type "Float (double-precision)") (InputAction :type "InputAction Object Reference" :default "/Game/Player/Controls/IA_Shoot.IA_Shoot"))
  (:`Triggered`
    (`/Game/Enemies/AC_HealthComponent.DeductHealth` (`self.AC_HealthComponent`) (`self.Damage`))
    (`self.OnDeath`)))

(event `self.ReceiveBeginPlay`)

(event `OnDeath`
  (while (<= (`self.Successors`) 0)
    (`|SpawnActorFromClass` "BP_BubbleEnemy_C" (`KismetMathLibrary.MakeTransform` (`self.K2_GetActorLocation`)) "Undefined" "MultiplyWithRoot" null 2 null)
    (set `self.Successors` (- (`self.Successors`) 1))))

(fn `UserConstructionScript`)