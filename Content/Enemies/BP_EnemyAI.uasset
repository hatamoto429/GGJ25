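; Enemy AI controller that steers its controlled pawn toward a player character.
; Tick calls TrackNearestPlayer, which despite its name always issues AIMoveTo toward player 0.
; GetClosestPlayer loops over BP_BubbleChar actors with nested distance checks against player pawns, but nothing shown calls it and the move ignores its result.
; BeginPlay calls SetTimerByFunctionName with no function specified.
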(event `self.ReceiveBeginPlay`
  (`KismetSystemLibrary.K2_SetTimer` null))

(event `self.ReceiveTick`
  (params (DeltaSeconds :type "Float (single-precision)"))
  (`self.Track Nearest Player`))

(event `Track Nearest Player`
  (`|AIMoveTo` (`self.K2_GetPawn`) (0.0 0.0 0.0) (`GameplayStatics.GetPlayerCharacter` 0)))

(event `GetClosestPlayer`
  (bind _outactors (`GameplayStatics.GetAllActorsOfClass` "/Game/Player/BP_BubbleChar.BP_BubbleChar_C"))
  (set `self.CLosestPlayer` (`|GetArrayItem` _outactors))
  (for (_array_element _array_index) _outactors
    (if (!= _array_index 0)
      (if (`KismetSystemLibrary.IsValid` (`GameplayStatics.GetPlayerPawn` 1))
        (if (< (`self.GetDistanceTo` (`self.CLosestPlayer`) (`GameplayStatics.GetPlayerPawn` 0)) (`self.GetDistanceTo` (`self.CLosestPlayer`) (`GameplayStatics.GetPlayerPawn` 1)))
          (set `self.CLosestPlayer` _array_element)
          (elif (`KismetSystemLibrary.IsValid` (`GameplayStatics.GetPlayerPawn` 2))
            (if (< (`self.GetDistanceTo` (`self.CLosestPlayer`) (`GameplayStatics.GetPlayerPawn` 0)) (`self.GetDistanceTo` (`self.CLosestPlayer`) (`GameplayStatics.GetPlayerPawn` 2)))
              (set `self.CLosestPlayer` _array_element)
              (elif (`KismetSystemLibrary.IsValid` (`GameplayStatics.GetPlayerPawn` 2))
                (if (< (`self.GetDistanceTo` (`self.CLosestPlayer`) (`GameplayStatics.GetPlayerPawn` 0)) (`self.GetDistanceTo` (`self.CLosestPlayer`) (`GameplayStatics.GetPlayerPawn` 3)))
                  (set `self.CLosestPlayer` _array_element)
                  (elif (`KismetSystemLibrary.IsValid` (`GameplayStatics.GetPlayerPawn` 2))
                    (if (< (`self.GetDistanceTo` (`self.CLosestPlayer`) (`GameplayStatics.GetPlayerPawn` 0)) (`self.GetDistanceTo` (`self.CLosestPlayer`) (`GameplayStatics.GetPlayerPawn` 4)))
                      (set `self.CLosestPlayer` _array_element))))))))))))

(fn `UserConstructionScript`)