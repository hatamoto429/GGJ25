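; BP_WhiteHole_Push is a white hole actor that pushes nearby physics objects away from itself.
; Every tick, ApplyFoces gathers components overlapping GravityInfluence and applies a force to those simulating physics.
; The force points away from the actor's center, scales with GravityStrenght and fades linearly to zero at a fixed radius.
; Its vertical component is amplified relative to the horizontal axes.
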(event `self.ReceiveTick`
  (params (DeltaSeconds :type "Float (single-precision)"))
  (`self.ApplyFoces`))

(fn `ApplyFoces`
  (bind _returnvalue (`self.K2_GetActorLocation`))
  (for _array_element (`PrimitiveComponent.GetOverlappingComponents` (`self.GravityInfluence`))
    (if (`SceneComponent.IsSimulatingPhysics` _array_element "None")
      (bind _returnvalue_2 (`SceneComponent.K2_GetComponentLocation` _array_element))
      (`PrimitiveComponent.AddForce` _array_element (* (* (`KismetMathLibrary.GetDirectionUnitVector` _returnvalue_2 _returnvalue) (* (- 1.0 (`KismetMathLibrary.FClamp` (/ (`KismetMathLibrary.Vector_Distance` _returnvalue_2 _returnvalue) 5000.0))) 5000.0) (1.0 1.0 5.0) (`self.GravityStrenght`)) -1.0) "None" false))))

(fn `UserConstructionScript`)