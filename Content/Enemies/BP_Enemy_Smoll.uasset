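; Small bubble enemy that wanders by hovering and moves toward the player once PawnSensing spots them.
; A looping timeline lerps it between random XY targets at constant height, and is not stopped during the chase.
; Player contact kills them and fires a radial projectile ring; lethal damage splits it into BP_BubbleEnemyBig children.
; Construction picks one of three random materials; the scale pulse is unconnected.
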(event `InitLocation`
  ; Reference Setter
  (set `self.OwnLocation` (`self.K2_GetActorLocation`)))

(event `TargetPlayerLocation`
  ; Reference Setter
  (set `self.PlayerLocation` (`self.K2_GetActorLocation` (`self.TargetedPlayer`))))

(event `Pulsate`
  ;[0 0.8125 0.6724 0.5] Pulsating
)

(event `self.ReceiveBeginPlay`
  ;[0.1605 0.8802 0.1933 0.5] Begin Play
  (`|ExecutionSequence`
    (:`then_0`
      (set `self.IsPassive` true))
    (:`then_1`
      (`self.InitLocation`)
      (`self.SetTargetLocation`))
    (:`then_2`
      (`self.Pulsate`)
      (`self.Hovering`))))

(event `Hovering`
  ;[0 0.8125 0.6724 0.5] Hovering
  (`/Engine/EditorBlueprintResources/StandardMacros.DoOnce` false :!label _label
    (:`Completed`
      (bind (_direction _hover) (`Timeline|Hover`)
        (:`Update`
          (`self.K2_SetActorLocation` (`KismetMathLibrary.VLerp` (`self.OwnLocation`) (`self.TargetLocation`) _hover)))
        (:`Finished`
          (`self.InitLocation`)
          (`self.SetTargetLocation`)
          (`self.Hovering`)
          (goto _label :!via `Reset`))))))

(event `self.PawnSensing.OnSeePawn`
  (params (Pawn :type "Pawn Object Reference"))
  ;[0.901 0.05116 0 0.5] Target
  (bind _asbp_bubble_char (cast `/Game/Player/BP_BubbleChar` Pawn)
    (:`then`
      (set `self.IsPassive` false)
      (`|AIMoveTo` self (0.0 0.0 0.0) _asbp_bubble_char 3.0))
    (:`CastFailed`
      (`KismetSystemLibrary.PrintString` "Hello"))))

(event `SetTargetLocation`
  (bind _returnvalue (`KismetMathLibrary.RandomFloatInRange` -300.0 300.0))
  (bind (_ownlocation_x _ownlocation_y _ownlocation_z) (`KismetMathLibrary.BreakVector` (`self.OwnLocation`)))
  ;[0 0.8125 0.6724 0.5] Hovering Movement
  (`|ExecutionSequence`
    (:`then_0`
      (bind _output_get (set `self.MovementOffsetX` (+ _ownlocation_x _returnvalue))))
    (:`then_1`
      (bind _output_get_2 (set `self.MovementOffsetY` (+ _ownlocation_y _returnvalue))))
    (:`then_2`
      (bind _output_get_3 (set `self.MovementOffsetZ` (+ 0.0 _ownlocation_z)))))
  (set `self.TargetLocation` (`KismetMathLibrary.MakeVector` _output_get _output_get_2 _output_get_3)))

(event `self.Collision.OnComponentBeginOverlap`
  (params (OverlappedComponent :type "PrimitiveComponent Object Reference") (OtherActor :type "Actor Object Reference") (OtherComp :type "PrimitiveComponent Object Reference") (OtherBodyIndex :type Integer) (bFromSweep :type Boolean) (SweepResult :type "HitResult Structure (by ref)"))
  ; Hit Check - Player Pawn
  (bind _asbp_bubble_char (cast `/Game/Player/BP_BubbleChar` OtherActor))
  (`self.Collision: Player` _asbp_bubble_char))

(event `self.ReceiveAnyDamage`
  (params (Damage :type "Float (single-precision)") (DamageType :type "DamageType Object Reference") (InstigatedBy :type "Controller Object Reference") (DamageCauser :type "Actor Object Reference"))
  ; On Damaged
  (set `self.EnemyHealth` (- (`self.EnemyHealth`) Damage))
  (if (<= (`self.EnemyHealth`) 0.0)
    (`self.Split`)
    (`self.K2_DestroyActor`)))

(event `Spawn Projectiles`
  ;[0.7552 0.1934 0.6201 0.5] Projectiles
  (`GameplayStatics.PlaySound2D` "/Game/SpacePewPew/Audio/376694__daleonfire__laser.376694__daleonfire__laser" 1.0 1.0 0.0 null null)
  (for _index (range (`self.ProjectileAmount`))
    (bind _returnvalue (`KismetMathLibrary.ComposeRotators` (`self.K2_GetActorRotation`) (`KismetMathLibrary.MakeRotator` 0.0 0.0 (* _index (/ 360 (`self.ProjectileAmount`))))))
    (`|SpawnActorFromClass` "/Game/Enemies/BP_EnemyProjectile.BP_EnemyProjectile_C" (`KismetMathLibrary.MakeTransform` (+ (`self.K2_GetActorLocation`) (* (`KismetMathLibrary.GetForwardVector` _returnvalue) 100)) _returnvalue) "Undefined" "MultiplyWithRoot" null 100.0 null)))

(event `Collision: Player`
  (params (Player :type "/Game/Player/BP_BubbleChar Object Reference"))
  ; Hit Action
  (`/Game/Player/BP_BubbleChar.KillPlayer` Player)
  (`self.Spawn Projectiles`)
  (`self.K2_DestroyActor`))

(event `Split`
  (bind (_returnvalue_x _returnvalue_y _returnvalue_z) (`KismetMathLibrary.BreakVector` (`self.K2_GetActorLocation`)))
  (bind _returnvalue (`KismetMathLibrary.RandomFloatInRange` 100.0 200.0))
  ; Hit Action
  (for _ (range 1 (+ (`self.ChildCount`) 1))
    (`|SpawnActorFromClass` "/Game/Enemies/BP_BubbleEnemyBig.BP_BubbleEnemyBig_C" (`KismetMathLibrary.MakeTransform` (`KismetMathLibrary.MakeVector` (- _returnvalue_x _returnvalue) (+ _returnvalue_y _returnvalue) _returnvalue_z)) "Undefined" "MultiplyWithRoot" null (0.0 0.0 0.0) (0.0 0.0 0.0) (0.0 0.0 0.0) null)))

(event `DestroyActor`
  ;[1 0.02207 0 0.5] Death
  (`self.K2_DestroyActor`))

(fn `UserConstructionScript`
  ; Select one out of three random materials
  (bind _returnvalue (`KismetMaterialLibrary.CreateDynamicMaterialInstance` (`|GetArrayItem` (`self.Material`) (`KismetMathLibrary.RandomInteger` 3))))
  (`PrimitiveComponent.SetMaterial` (`self.Bubble`) 0 _returnvalue))